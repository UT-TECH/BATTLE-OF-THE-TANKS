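; Allied tank pawn Blueprint that wires its barrel, turret and tracks into aiming and movement components on BeginPlay.
; Input axes drive track movement and rotate an azimuth gimbal and spring arm for the camera.
; TankAiming.Fire runs every Tick as well as on the Fire Cannon input, which also plays a cannon sound.
; A widget component's HealthBar_UI receives a reference to the tank.
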(event EventTick
  (params (DeltaSeconds :type Float%20%28single-precision%29))
  (Class|TankAimingComponent|Fire (Variables|Default|GetTankAiming)))

(event Collision|EventActorBeginOverlap
  (params (OtherActor :type Actor%20Object%20Reference)))

(event EventBeginPlay
  (Class|TankAimingComponent|Initialise (Variables|Default|GetTankAiming) (Variables|Default|GetTankBarrel) (Variables|Default|GetTankTurret))
  (Class|TankMovementComponent|Initialise (Variables|Default|GetTankMovement) (Variables|Default|GetLeftTrack) (Variables|Default|GetRightTrack))
  (CallFunction|InitialiseHealthBarWidget))

(event Input|ActionEvents|InputActionFireCannon
  (params (Key :type Key%20Structure))
  ;[1 1 1] firing input
  (:Pressed
    (Audio|PlaySound2D "/Game/TANK_01/Assets/SoundEffects/Cannon+2.Cannon+2" 1.0 1.0 0.0 0 0)
    (Class|TankAimingComponent|Fire (Variables|Default|GetTankAiming))))

(event Input|AxisEvents|InputAxisAimAzimuth
  (params (AxisValue :type Float%20%28single-precision%29))
  ;[1 1 1] Camera Input System
  (Transformation|AddLocalRotation (Variables|Default|GetAzimuth%20Gimbal) (Math|Rotator|MakeRotator 0.0 0.0 (* AxisValue (Utilities|Time|GetWorldDeltaSeconds) 1e+02)) false false))

(event Input|AxisEvents|InputAxisAimElevation
  (params (AxisValue :type Float%20%28single-precision%29))
  ;[1 1 1] Camera Input System
  (Transformation|AddLocalRotation (Variables|Default|GetSpringArm) (Math|Rotator|MakeRotator 0.0 (* AxisValue (Utilities|Time|GetWorldDeltaSeconds) 1e+02) 0.0) false false))

(event Input|AxisEvents|InputAxisTurnRight
  (params (AxisValue :type Float%20%28single-precision%29))
  (Class|TankMovementComponent|IntendTurnRight (Variables|Default|GetTankMovement) AxisValue))

(event Input|AxisEvents|InputAxisMoveForward
  (params (AxisValue :type Float%20%28single-precision%29))
  (Class|TankMovementComponent|IntendMoveForward (Variables|Default|GetTankMovement) AxisValue))

(fn ConstructionScript)

(fn InitialiseHealthBarWidget
  (bind _ashealth_bar_ui (Utilities|Casting|CastToHealthBar_UI (UserInterface|GetUserWidgetObject (Variables|Default|GetWidget))))
  (Variables|/Game/Blueprints/UI_Blueprints/HealthBar_UI.HealthBar_UI_C|SetMyTank _ashealth_bar_ui self)
  (return))